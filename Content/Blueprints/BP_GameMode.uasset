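; BP_GameMode is the game mode that tracks score, top score, enemy count and kills, and handles game flow.
; It creates the player HUD, game-over screen and pause menu, switching pause state, input mode and cursor.
; Helper functions play world camera shakes, open levels or the ship selector, and pass ship mesh and material to the game instance.
; Score load and save hooks run on BeginPlay and EndPlay but are empty.
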(event EventBeginPlay
  (CallFunction|LoadScore)
  (CallFunction|SetScore))

(event EventTick
  (params (DeltaSeconds :type Float%20%28single-precision%29)))

(event EventEndPlay
  (params (EndPlayReason :type EEndPlayReason%20Enum :default "Destroyed"))
  (CallFunction|SaveScore))

(fn ConstructionScript)

(fn LoadScore)

(fn SaveScore)

(fn SetScore
  (params (Additional%20Value :type Integer))
  (bind _output_get (Variables|Default|SetScore (+ Additional%20Value (Variables|Default|GetScore))))
  (if (>= _output_get (Variables|Default|GetTopScore))
    (Variables|Default|SetTopScore (Variables|Default|GetScore))))

(fn UpdateEnemyCount
  (params (Additional%20value :type Integer))
  (Variables|Default|SetEnemyCount (+ Additional%20value (Variables|Default|GetEnemyCount))))

(fn CameraShake
  (params (Shake :type Camera%20Shake%20Class%20Reference) (Epicenter :type Vector))
  (Camera|PlayWorldCameraShake Shake Epicenter 0.0 1e+03))

(fn GameOver
  (bind _returnvalue (Game|GetPlayerController 0))
  (bind _returnvalue_2 (UserInterface|CreateWidget "/Game/Blueprints/UI/GameOverUIWidget_BP.GameOverUIWidget_BP_C"))
  (bind _output_get (LocalVariables|SetGameEndWidget _returnvalue_2))
  (UserInterface|Viewport|AddtoViewport _output_get 0)
  (Variables|/Script/Engine.PlayerController|SetbShowMouseCursor _returnvalue true)
  (Input|SetInputModeUIOnly _returnvalue (LocalVariables|GetGameEndWidget) "DoNotLock"))

(fn EnemyKilled
  (Math|Integer|IncrementInt (Variables|Default|GetEmeniesKill)
    (:%20%20
      (CallFunction|UpdateEnemyCount -1))))

(fn PauseGame
  (bind _returnvalue (Game|GetPlayerController 0))
  (Game|SetGamePaused true)
  (Utilities|IsValid (Variables|Default|GetPauseMenu)
    (:Is%20Valid
      _)
    (:Is%20Not%20Valid
      (bind _returnvalue_2 (UserInterface|CreateWidget "/Game/Blueprints/UI/PauseMenuWidget_BP.PauseMenuWidget_BP_C" _returnvalue))
      (bind _output_get (Variables|Default|SetPauseMenu _returnvalue_2))))
  (UserInterface|Viewport|AddtoViewport _output_get 0)
  (Input|SetInputModeUIOnly _returnvalue _output_get "DoNotLock")
  (bind _output_get_2 (Variables|/Script/Engine.PlayerController|SetbShowMouseCursor _returnvalue true))
  (Variables|Default|SetIsPause _output_get_2))

(fn UnpauseGame
  (bind _returnvalue (Game|GetPlayerController 0))
  (bind _pausemenu (Variables|Default|GetPauseMenu))
  (Game|SetGamePaused false)
  (Utilities|IsValid _pausemenu
    (:Is%20Valid
      (Widget|RemovefromParent _pausemenu))
    (:Is%20Not%20Valid
      (bind _foundwidgets (Widget|GetAllWidgetsOfClass "/Game/Blueprints/UI/PauseMenuWidget_BP.PauseMenuWidget_BP_C" true))
      (Widget|RemovefromParent _foundwidgets)))
  (Input|SetInputModeGameOnly _returnvalue)
  (bind _output_get (Variables|/Script/Engine.PlayerController|SetbShowMouseCursor _returnvalue false))
  (Variables|Default|SetIsPause _output_get))

(fn LoadPlayerUI
  (Utilities|IsValid (Variables|Default|GetUI)
    (:Is%20Not%20Valid
      (bind _returnvalue (UserInterface|CreateWidget "/Game/Blueprints/UI/UIWidget_BP.UIWidget_BP_C"))
      (bind _output_get (Variables|Default|SetUI _returnvalue))
      (UserInterface|Viewport|AddtoViewport _output_get 0))))

(fn LoadSelectedShip
  (Game|OpenLevel(byName) "ShipSelecter"))

(fn SetPlayerStyle
  (params (Mesh :type Static%20Mesh%20Object%20Reference) (Material :type Material%20Interface%20Object%20Reference))
  (bind _asmy_game_instance_bp (Utilities|Casting|CastToMyGameInstance_BP (Game|GetGameInstance)))
  (Default|SetrStyle _asmy_game_instance_bp Mesh Material))

(fn LoadLevel
  (params (LevelName :type Name))
  (Game|OpenLevel(byName) LevelName))