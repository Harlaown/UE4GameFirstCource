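; Player pawn for a shooter that moves in the XZ plane, fires projectiles and ends the game on death.
; A spin-and-rise timeline plays on spawn, then enables firing via MoveEnabled.
; Input axes feed interpolated speeds into swept moves and mesh yaw, while held fire buttons loop timers for single primary and paired secondary shots.
; Damage shakes the camera through BP_GameMode; IsAlive actually returns true at zero health, triggering Died.
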(event Custom|PrimaryFire
  ;[1 1 1] Primary Fire
  (CallFunction|PrimaryFire (Transformation|GetWorldTransform (Variables|Default|GetProjectileSpawn))))

(event Custom|SecondFire
  ;[1 1 1] Secondary Fire
  (CallFunction|SecondaryFire (Transformation|GetWorldTransform (Variables|Default|GetProjectileRight)))
  (CallFunction|SecondaryFire (Transformation|GetWorldTransform (Variables|Default|GetProjectileLeft))))

(event EventBeginPlay
  ;[1 1 1] Player Spawn Animation
  (bind _asbp_game_mode (Utilities|Casting|CastToBP_GameMode (Game|GetGameMode)))
  (Variables|Default|SetBP_GameMode _asbp_game_mode)
  (Variables|Default|SetYaw (.Yaw (Math|Rotator|BreakRotator (Transformation|GetActorRotation))))
  (Variables|Default|SetSpawnLocation (Transformation|GetActorLocation))
  (bind _speed (Timeline|SpawnAnimation Play)
    (:Update
      (Transformation|SetActorLocation (Math|Vector|Lerp(Vector) (Variables|Default|GetSpawnLocation) (+ (Variables|Default|GetSpawnLocation) "0, 0,60.000000") _speed) false false)
      (CallFunction|Spin _speed (Variables|Default|GetSpawnSpeenCount)))
    (:Finished
      (Variables|Default|SetMoveEnabled true))))

(event EventTick
  (params (DeltaSeconds :type Float%20%28single-precision%29))
  (bind _playermesh (Variables|Default|GetPlayerMesh))
  ;[1 1 1] Movement update
  (Variables|Default|SetDeltaSeconds DeltaSeconds)
  (CallFunction|Moveto (Math|Vector|MakeVector (Variables|Default|GetHorizontalSpeed) 0.0 0.0))
  (CallFunction|Moveto (Math|Vector|MakeVector 0.0 0.0 (Variables|Default|GetVerticalSpeed)))
  (Utilities|IsValid self
    (:Is%20Valid
      (bind _newplayerrotator (CallFunction|YawRotate (Variables|Default|GetDeltaSeconds) (Variables|Default|GetYaw) (Variables|Default|GetHorizontalSpeed) (Variables|/Script/Engine.SceneComponent|GetRelativeRotation _playermesh) 8e+01))
      (Transformation|SetRelativeRotation _playermesh _newplayerrotator false false))))

(event Game|Damage|EventAnyDamage
  (params (Damage :type Float%20%28single-precision%29) (DamageType :type Damage%20Type%20Object%20Reference) (InstigatedBy :type Controller%20Object%20Reference) (DamageCauser :type Actor%20Object%20Reference))
  ;[1 1 1] Take Damage
  (CallFunction|AplayDamage Damage)
  (CallFunction|CameraShake "/Game/Blueprints/BP_CamShakeSmall.BP_CamShakeSmall_C")
  (if (CallFunction|IsAlive)
    (CallFunction|Died)))

(event Input|ActionEvents|InputActionPrimaryFire
  (params (Key :type Key%20Structure :default "None"))
  ;[1 1 1] Primary Fire
  (:Pressed
    (if (Variables|Default|GetMoveEnabled)
      (bind _returnvalue (Utilities|Time|SetTimerbyEvent (delegate Custom|PrimaryFire) 0.1 true))
      (bind _output_get (Variables|Default|SetPrimeFireTimer _returnvalue))))
  (:Released
    (Utilities|Time|ClearandInvalidateTimerbyHandle _output_get)))

(event Input|ActionEvents|InputActionSecondaryFire
  (params (Key :type Key%20Structure :default "None"))
  ;[1 1 1] Secondary Fire
  (:Pressed
    (if (Variables|Default|GetMoveEnabled)
      (bind _returnvalue (Utilities|Time|SetTimerbyEvent (delegate Custom|SecondFire) 0.4 true))
      (bind _output_get (Variables|Default|SetSecondaryFireTimer _returnvalue))))
  (:Released
    (Utilities|Time|ClearandInvalidateTimerbyHandle _output_get)))

(event Input|AxisEvents|InputAxisMoveUp
  (params (AxisValue :type Float%20%28single-precision%29))
  ;[1 1 1] Input
  (bind _directionspeed (CallFunction|GetPlayerSpeedbyInputPosition (Variables|Default|GetVerticalSpeed) AxisValue 12.0))
  (Variables|Default|SetVerticalSpeed _directionspeed))

(event Input|AxisEvents|InputAxisMoveRight
  (params (AxisValue :type Float%20%28single-precision%29))
  ;[1 1 1] Input
  (bind _directionspeed (CallFunction|GetPlayerSpeedbyInputPosition (Variables|Default|GetHorizontalSpeed) AxisValue 12.0))
  (Variables|Default|SetHorizontalSpeed _directionspeed))

(fn ConstructionScript
  (Variables|Default|SetHealth (Variables|Default|GetMaxHealth)))

(fn GetPlayerSpeedbyInputPosition
  (params (CurrentSpeed :type Float%20%28single-precision%29) (Direction :type Float%20%28single-precision%29) (InetrpalateSpeed :type Float%20%28single-precision%29))
  (return (Math|Interpolation|FInterpTo CurrentSpeed (* (* Direction (Variables|Default|GetMovementSpeed)) (Variables|Default|GetDeltaSeconds)) (Variables|Default|GetDeltaSeconds) InetrpalateSpeed)))

(fn Moveto
  (params (Position :type Vector))
  (Transformation|SetActorLocation (+ (Transformation|GetActorLocation) Position) true false))

(fn YawRotate
  (params (Delta%20second :type Float%20%28single-precision%29%20%28by%20ref%29) (Yaw :type Float%20%28single-precision%29%20%28by%20ref%29) (Horizontal%20speed :type Float%20%28single-precision%29%20%28by%20ref%29) (PlayerRotator :type Rotator) (Iterp%20Speed :type Float%20%28single-precision%29))
  (return (Class|KismetMathLibrary|RInterptoConstant PlayerRotator (Math|Rotator|MakeRotator 0.0 0.0 (+ Yaw (* Horizontal%20speed -7.0))) Delta%20second Iterp%20Speed)))

(fn Spin
  (params (Speed :type Float%20%28single-precision%29%20%28by%20ref%29) (SpeenCount :type Integer%20%28by%20ref%29))
  (Transformation|SetRelativeRotation (Variables|Default|GetPlayerMesh) (Math|Rotator|Lerp(Rotator) "0, 0, 0" (Math|Rotator|MakeRotator 0.0 0.0 (+ (Variables|Default|GetYaw) (* SpeenCount 3.6e+02))) Speed) false false))

(fn PrimaryFire
  (params (SpawnTransform :type Transform))
  (Game|SpawnActorfromClass "/Game/Blueprints/Projectile/Player/BP_ProjectailPlayerPrim.BP_ProjectailPlayerPrim_C" SpawnTransform "AlwaysSpawn" 0 (LocalVariables|GetprojectileColor) self))

(fn SecondaryFire
  (params (SpawnTransform :type Transform))
  (Game|SpawnActorfromClass "/Game/Blueprints/Projectile/Player/BP_ProjectailPlayerSecond.BP_ProjectailPlayerSecond_C" SpawnTransform "AlwaysSpawn" 0 (LocalVariables|GetColor) 0))

(fn StopAllTimer
  (Utilities|Time|ClearandInvalidateTimerbyHandle (Variables|Default|GetPrimeFireTimer))
  (Utilities|Time|ClearandInvalidateTimerbyHandle (Variables|Default|GetSecondaryFireTimer)))

(fn CameraShake
  (params (Shake :type Camera%20Shake%20Class%20Reference))
  (Default|CameraShake (Variables|Default|GetBP_GameMode) Shake (Transformation|GetActorLocation))
  (return))

(fn Died
  (Effects|SpawnEmitteratLocation "/Game/Assets/Particles/P_Pixel_Explosion.P_Pixel_Explosion" (Transformation|GetActorLocation))
  (Audio|PlaySoundatLocation 0 "0, 0, 0" "0, 0, 0" 1.0 1.0 0.0 0 0 0)
  (CallFunction|CameraShake "/Game/Blueprints/BP_CamShake.BP_CamShake_C")
  (Default|GameOver (Variables|Default|GetBP_GameMode))
  (CallFunction|StopAllTimer)
  (Actor|DestroyActor))

(fn IsAlive
  (return (<= (Variables|Default|GetHealth) 0.0)))

(fn AplayDamage
  (params (Damage :type Float%20%28single-precision%29))
  (Variables|Default|SetHealth (Math|Float|Clamp(Float) (- (Variables|Default|GetHealth) Damage) 0.0 (Variables|Default|GetMaxHealth))))