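; BP_ProjectaileEnemybase is an enemy projectile, apparently a base class, that damages the player on hit.
; The construction script creates a dynamic material tinted by ProjectailColor, scales the Projectile component, and feeds Speed into the movement component's max and initial speed.
; BeginPlay reapplies the color.
; A component hit applies Damage only to BP_Player, then destroys the projectile whatever it struck.
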(event OnComponentHit(Projectile)
  (params (HitComponent :type Primitive%20Component%20Object%20Reference) (OtherActor :type Actor%20Object%20Reference) (OtherComp :type Primitive%20Component%20Object%20Reference) (NormalImpulse :type Vector :default "0, 0, 0") (Hit :type Hit%20Result%20Structure%20%28by%20ref%29))
  (bind _asbp_player (Utilities|Casting|CastToBP_Player OtherActor)
    (:then
      (Game|Damage|ApplyDamage _asbp_player (Variables|Default|GetDamage) 0 0))
    (:CastFailed
      _))
  (Actor|DestroyActor))

(event EventBeginPlay
  (Rendering|Material|SetVectorParameterValue (Variables|Default|GetProjectailmaterial) "Color" (Variables|Default|GetProjectail%20Color) :!class /Script/Engine.MaterialInstanceDynamic))

(fn ConstructionScript
  (bind _projectilemovement (Variables|Default|GetProjectileMovement))
  (bind _returnvalue (Rendering|Material|CreateDynamicMaterialInstance (Variables|Default|GetProjectile) 0 0 "None" :!class /Script/Engine.PrimitiveComponent))
  (bind _output_get (Variables|Default|SetProjectailmaterial _returnvalue))
  (Rendering|Material|SetVectorParameterValue _output_get "Color" (Variables|Default|GetProjectail%20Color) :!class /Script/Engine.MaterialInstanceDynamic)
  (Transformation|SetWorldScale3D (Variables|Default|GetProjectile) (Variables|Default|GetScale))
  (bind _output_get_2 (Variables|/Script/Engine.ProjectileMovementComponent|SetMaxSpeed _projectilemovement (Variables|Default|GetSpeed)))
  (Variables|/Script/Engine.ProjectileMovementComponent|SetInitialSpeed _projectilemovement _output_get_2))