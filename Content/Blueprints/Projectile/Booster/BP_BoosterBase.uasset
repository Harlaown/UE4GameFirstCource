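; Base booster projectile that boosts a BP_Player it hits.
; On a component hit with a player, it passes ActivePeriod to the player's Boosted function and destroys itself; other hits are ignored.
; A timer started at BeginPlay destroys it after a short lifetime regardless.
; The construction script applies the Color variable through a dynamic material instance and sets the projectile's world scale from Scale.
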(event OnComponentHit(Projectile)
  (params (HitComponent :type Primitive%20Component%20Object%20Reference) (OtherActor :type Actor%20Object%20Reference) (OtherComp :type Primitive%20Component%20Object%20Reference) (NormalImpulse :type Vector :default "0, 0, 0") (Hit :type Hit%20Result%20Structure%20%28by%20ref%29))
  (bind _asbp_player (Utilities|Casting|CastToBP_Player OtherActor))
  (Default|Boosted _asbp_player (Variables|Default|GetActivePeriod))
  (Actor|DestroyActor))

(event Custom|Destroy
  (Actor|DestroyActor))

(event EventBeginPlay
  (|CallParentFunction)
  (Utilities|Time|SetTimerbyEvent (delegate Custom|Destroy) 2.0))

(event Collision|EventActorBeginOverlap
  (params (OtherActor :type Actor%20Object%20Reference))
  (|CallParentFunction 0))

(event EventTick
  (params (DeltaSeconds :type Float%20%28single-precision%29))
  (|CallParentFunction 0.0))

(fn ConstructionScript
  (bind _returnvalue (Rendering|Material|CreateDynamicMaterialInstance (Variables|Default|GetProjectile) 0 0 "None" :!class /Script/Engine.PrimitiveComponent))
  (Rendering|Material|SetVectorParameterValue _returnvalue "Color" (Variables|Default|GetColor) :!class /Script/Engine.MaterialInstanceDynamic)
  (Transformation|SetWorldScale3D (Variables|Default|GetProjectile) (Variables|Default|GetScale)))