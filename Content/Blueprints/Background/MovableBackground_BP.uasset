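; MovableBackground_BP is a vertically scrolling, endlessly repeating background built from two planes, TOP and BOTTOM.
; Each tick it moves the root along the up axis by Speed, scaled by delta time.
; Either plane dropping below minus VerticalSize in world Z jumps up two heights, leapfrogging the other.
; The construction script derives VerticalSize from the root's Y scale and creates a dynamic material for each plane.
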(event EventBeginPlay)

(event Collision|EventActorBeginOverlap
  (params (OtherActor :type Actor%20Object%20Reference)))

(event EventTick
  (params (DeltaSeconds :type Float%20%28single-precision%29))
  (bind _output_get (Variables|Default|SetDeltaTime DeltaSeconds))
  (CallFunction|TranslatePlane (Variables|Default|GetDefaultSceneRoot) (Variables|Default|GetSpeed) _output_get)
  (CallFunction|RepeatingBackground (Variables|Default|GetBOTTOM))
  (CallFunction|RepeatingBackground (Variables|Default|GetTOP)))

(fn ConstructionScript
  (Variables|Default|SetVerticalSize (* 100 (.y (Transformation|GetWorldScale (Variables|Default|GetDefaultSceneRoot)))))
  (bind _returnvalue (Rendering|Material|CreateDynamicMaterialInstance (Variables|Default|GetBOTTOM) 0 (Variables|Default|GetBotMaterial) "None" :!class /Script/Engine.PrimitiveComponent))
  (Variables|Default|SetDynamicBotMaterial _returnvalue)
  (bind _returnvalue_2 (Rendering|Material|CreateDynamicMaterialInstance (Variables|Default|GetTOP) 0 (Variables|Default|GetTopMaterial) "None" :!class /Script/Engine.PrimitiveComponent))
  (Variables|Default|SetDynamicTopMaterial _returnvalue_2))

(fn TranslatePlane
  (params (Component :type Scene%20Component%20Object%20Reference%20%28by%20ref%29) (Speed :type Float%20%28single-precision%29%20%28by%20ref%29) (Deltatime :type Float%20%28single-precision%29%20%28by%20ref%29))
  (Transformation|SetRelativeLocation Component (+ (.location (Transformation|GetRelativeTransform Component)) (* (* (Math|Vector|VectorUp) Speed) Deltatime)) true false))

(fn RepeatingBackground
  (params (Background :type Scene%20Component%20Object%20Reference%20%28by%20ref%29))
  (if (< (.z (Transformation|GetWorldLocation Background)) (* (Variables|Default|GetVerticalSize) -1.0))
    (Transformation|SetWorldLocation Background (+ (Transformation|GetWorldLocation Background) (Math|Vector|MakeVector 0.0 0.0 (* (Variables|Default|GetVerticalSize) 2.0))) false false)))