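; SelectionShip is the preview actor for a ship selection screen, where the player picks a ship mesh and color material.
; On BeginPlay it creates the selector widget, binds its events, switches to UI-only input and copies the widget's color-to-material map.
; Next and Prev cycle the mesh array with wraparound, while color changes swap material slot 0.
; Apply passes the chosen mesh and material to BP_GameMode as the player style.
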(event Custom|OnNext
  (bind _result (Math|Integer|IncrementInt (Variables|Default|GetIndex))
    (:%20%20
      (if (>= _result (Utilities|Array|Length (Variables|Default|GetMeshes)))
        (bind _output_get (Variables|Default|SetIndex 0))
        (CallFunction|SetMesh _output_get)
        (else
          (CallFunction|SetMesh (Variables|Default|GetIndex)))))))

(event Custom|OnPrev
  (bind _result (Math|Integer|DecrementInt (Variables|Default|GetIndex))
    (:%20%20
      (if (<= _result 0)
        (bind _output_get (Variables|Default|SetIndex (- (Utilities|Array|Length (Variables|Default|GetMeshes)) 1)))
        (CallFunction|SetMesh _output_get)
        (else
          (CallFunction|SetMesh (Variables|Default|GetIndex)))))))

(event Custom|OnColorChanged
  (bind _output_get (Variables|Default|SetSelectedColor (Variables|/Game/Blueprints/UI/SelecterUIWidget_BP.SelecterUIWidget_BP_C|GetSelectedItem (Variables|Default|GetUI))))
  (CallFunction|SetColor _output_get))

(event Custom|OnApplay
  (Utilities|IsValid (Variables|Default|GetGM)
    (:Is%20Valid
      _)
    (:Is%20Not%20Valid
      (bind _asbp_game_mode (Utilities|Casting|CastToBP_GameMode (Game|GetGameMode)))
      (bind _output_get (Variables|Default|SetGM _asbp_game_mode))))
  (Default|SetPlayerStyle _output_get (Utilities|Array|Get(acopy) (Variables|Default|GetMeshes) (Variables|Default|GetIndex)) (.Value (Utilities|Map|Find (Variables|Default|GetColorsMaterials) (Variables|Default|GetSelectedColor)))))

(event EventBeginPlay
  (bind _returnvalue (Game|GetPlayerController 0))
  (bind _returnvalue_2 (UserInterface|CreateWidget "/Game/Blueprints/UI/SelecterUIWidget_BP.SelecterUIWidget_BP_C" (Game|GetPlayerController 0)))
  (bind _output_get (Variables|Default|SetUI _returnvalue_2))
  (EventDispatchers|BindEventtoOnNext _output_get (delegate Custom|OnNext))
  (EventDispatchers|BindEventtoOnChangeSelectedColor _output_get (delegate Custom|OnColorChanged))
  (EventDispatchers|BindEventtoOnPrev _output_get (delegate Custom|OnPrev))
  (EventDispatchers|BindEventtoOnApplay (Variables|Default|GetUI) (delegate Custom|OnApplay))
  (UserInterface|Viewport|AddtoViewport (Variables|Default|GetUI) 0)
  (Input|SetInputModeUIOnly _returnvalue (Variables|Default|GetUI) "DoNotLock")
  (Variables|/Script/Engine.PlayerController|SetbShowMouseCursor _returnvalue true)
  (Variables|Default|SetColorsMaterials (Variables|/Game/Blueprints/UI/SelecterUIWidget_BP.SelecterUIWidget_BP_C|GetColorsMatireals (Variables|Default|GetUI)))
  (CallFunction|SetMesh (Variables|Default|GetIndex))
  (bind _keys (Utilities|Map|Keys (Variables|Default|GetColorsMaterials)))
  (bind _array_element (Utilities|Array|ForEachLoopwithBreak _keys :!label _label)
    (:LoopBody
      (bind _output_get_2 (Variables|Default|SetSelectedColor _array_element))
      (CallFunction|SetColor _output_get_2)
      (goto _label Break))))

(fn ConstructionScript)

(fn SetMesh
  (params (Index :type Integer%20%28by%20ref%29))
  (Components|StaticMesh|SetStaticMesh (Variables|Default|GetStaticMesh) (Utilities|Array|Get(acopy) (Variables|Default|GetMeshes) Index)))

(fn SetColor
  (params (Color :type String%20%28by%20ref%29))
  (bind _colorsmaterials (Variables|Default|GetColorsMaterials))
  (bind _value (Utilities|Map|Find _colorsmaterials Color))
  (Utilities|IsValid _value
    (:Is%20Valid
      (Rendering|Material|SetMaterial (Variables|Default|GetStaticMesh) 0 _value))))