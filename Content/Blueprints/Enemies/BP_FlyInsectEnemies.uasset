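; Flying insect enemy that flaps four wings with a timer-driven timeline and handles its death with effects, score and camera shake.
; As health falls past quarter thresholds, TakeDamage triggers EpicAttack, which spawns BP_FlyInsectSpecial "eggs" using a timeline-delayed loop.
; While any egg is alive the insect ignores damage, and its wings are tinted red through dynamic materials, with a looping timer refreshing the color.
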(event Custom|Wings
  ;[1 1 1] Start
  (Utilities|FlowControl|FlipFlop
    (:A
      (bind _angle (Timeline|Fly Play)
        (:Update
          (CallFunction|WingsFlying _angle))))
    (:B
      (Timeline|Fly Reverse))))

(event Custom|EpicAttack
  (params (Count :type Integer))
  ;[1 1 1] EpicAttack
  (if (not (>= (Variables|Default|GetCurrentIndex) Count)) :!label _label
    (bind _returnvalue (Game|SpawnActorfromClass "/Game/Blueprints/Enemies/BP_FlyInsectSpecial.BP_FlyInsectSpecial_C" (Math|Transform|MakeTransform (Transformation|GetWorldLocation (Variables|Default|GetProjecteilPosition)) "0, 0, 0" "0.125000,0.250000,0.250000") "Undefined" self "/Game/Assets/Meshes/Missiles/SM_MissileAlien.SM_MissileAlien" "/Game/Assets/Materials/Missiles/MissileAlien/M_MissileAlien_Red.M_MissileAlien_Red" "NewEnumerator0" 0))
    (Utilities|Array|Add (Variables|Default|GetSuperEggs) _returnvalue)
    (Math|Integer|IncrementInt (Variables|Default|GetCurrentIndex)
      (:%20%20
        (Variables|Default|SetIsEggLife true)
        (CallFunction|ChangeWingsSkin "(R=0.656250,G=0.019749,B=0.006692,A=1.000000)")
        (Timeline|Wait Play
          (:Finished
            (goto _label)))))))

(event Custom|ColorChange
  (Variables|Default|SetIsEpicAtack false)
  (bind _array_element (Utilities|Array|ForEachLoopwithBreak (Variables|Default|GetSuperEggs) :!label _label)
    (:LoopBody
      (if (Utilities|IsValid _array_element)
        (Variables|Default|SetIsEpicAtack true)
        (goto _label Break)))
    (:Completed
      (if (Variables|Default|GetIsEpicAtack)
        (CallFunction|ChangeWingsSkin "(R=0.656250,G=0.019749,B=0.006692,A=1.000000)")
        (else
          (CallFunction|ChangeWingsSkin "(R=1.000000,G=1.000000,B=1.000000,A=1.000000)"))))))

(event EventBeginPlay
  (bind _wing1 (Variables|Default|GetWing1))
  (bind _wingspositions (Variables|Default|GetWingsPositions))
  (bind _wing2 (Variables|Default|GetWing2))
  (bind _wing3 (Variables|Default|GetWing3))
  (bind _wing4 (Variables|Default|GetWing4))
  ;[1 1 1] Start
  (Utilities|Map|Add _wingspositions _wing1 (.roll (Variables|/Script/Engine.SceneComponent|GetRelativeRotation _wing1)))
  (Utilities|Map|Add _wingspositions _wing2 (.roll (Variables|/Script/Engine.SceneComponent|GetRelativeRotation _wing2)))
  (Utilities|Map|Add _wingspositions _wing3 (.roll (Variables|/Script/Engine.SceneComponent|GetRelativeRotation _wing3)))
  (Utilities|Map|Add _wingspositions _wing4 (.roll (Variables|/Script/Engine.SceneComponent|GetRelativeRotation _wing4)))
  (bind _returnvalue (Utilities|Time|SetTimerbyEvent (delegate Custom|Wings) 0.5 true))
  (Variables|Default|SetFlyingTimer _returnvalue)
  (|CallParentFunction)
  (Utilities|Time|SetTimerbyEvent (delegate Custom|ColorChange) 0.5 true))

(event EventTick
  (params (DeltaSeconds :type Float%20%28single-precision%29))
  ;[1 1 1] Tick
  (|CallParentFunction DeltaSeconds))

(event EventOnHit
  (params (Other :type Object%20Object%20Reference))
  ;[1 1 1] Hit
  (|CallParentFunction Other))

(fn ConstructionScript
  (|CallParentFunction)
  (bind _returnvalue (Rendering|Material|CreateDynamicMaterialInstance (Variables|Default|GetWing1) 0 0 "None" :!class /Script/Engine.PrimitiveComponent))
  (Utilities|Array|Add (Variables|Default|GetWingsMaterials) _returnvalue)
  (bind _returnvalue_2 (Rendering|Material|CreateDynamicMaterialInstance (Variables|Default|GetWing2) 0 0 "None" :!class /Script/Engine.PrimitiveComponent))
  (Utilities|Array|Add (Variables|Default|GetWingsMaterials) _returnvalue_2)
  (bind _returnvalue_3 (Rendering|Material|CreateDynamicMaterialInstance (Variables|Default|GetWing3) 0 0 "None" :!class /Script/Engine.PrimitiveComponent))
  (Utilities|Array|Add (Variables|Default|GetWingsMaterials) _returnvalue_3)
  (bind _returnvalue_4 (Rendering|Material|CreateDynamicMaterialInstance (Variables|Default|GetWing4) 0 0 "None" :!class /Script/Engine.PrimitiveComponent))
  (Utilities|Array|Add (Variables|Default|GetWingsMaterials) _returnvalue_4))

(fn WingsFlying
  (params (Alpha :type Float%20%28single-precision%29))
  (bind _wingspositions (Variables|Default|GetWingsPositions))
  (bind _keys (Utilities|Map|Keys _wingspositions))
  (for _array_element _keys
    (CallFunction|WingRotate _array_element (.Value (Utilities|Map|Find _wingspositions _array_element)) Alpha)))

(fn WingRotate
  (params (Wing :type Static%20Mesh%20Component%20Object%20Reference%20%28by%20ref%29) (StartAngle :type Float%20%28single-precision%29) (Alpha :type Float%20%28single-precision%29))
  (bind _relativerotation (Variables|/Script/Engine.SceneComponent|GetRelativeRotation Wing))
  (bind _angle (Variables|Default|GetAngle))
  (if (> StartAngle 0.0)
    (bind _output_get (LocalVariables|Settemp (+ StartAngle _angle)))
    (Transformation|SetRelativeRotation Wing (Math|Rotator|MakeRotator (Math|Float|Lerp StartAngle _output_get Alpha) (.pitch _relativerotation) (.yaw _relativerotation)) false false)
    (else
      (bind _output_get_2 (LocalVariables|Settemp (- StartAngle _angle)))
      (Transformation|SetRelativeRotation Wing (Math|Rotator|MakeRotator (Math|Float|Lerp StartAngle _output_get_2 Alpha) (.pitch _relativerotation) (.yaw _relativerotation)) false false))))

(fn CheckOpotinityEpicAttack
  (bind _hashsetepicattack (Variables|Default|GetHashSetEpicAttack))
  (bind _hashsetepicattack_2 (Variables|Default|GetHashSetEpicAttack))
  (bind _returnvalue (Utilities|Set|Contains _hashsetepicattack 75))
  (bind _returnvalue_2 (Utilities|Set|Contains _hashsetepicattack 50))
  (if (and (not _returnvalue) (<= (Variables|Default|GetHealth) (* (Variables|Default|GetMaxHealth) 0.75)))
    (CallFunction|EpicAttack 1)
    (Utilities|Set|Add _hashsetepicattack_2 75)
    (elif (Math|Boolean|ANDBoolean _returnvalue (not _returnvalue_2) (<= (Variables|Default|GetHealth) (* (Variables|Default|GetMaxHealth) 0.5)))
      (CallFunction|EpicAttack 2)
      (Utilities|Set|Add _hashsetepicattack_2 50)
      (elif (Math|Boolean|ANDBoolean (not (Utilities|Set|Contains _hashsetepicattack 25)) _returnvalue_2 _returnvalue (<= (Variables|Default|GetHealth) (* (Variables|Default|GetMaxHealth) 0.25)))
        (CallFunction|EpicAttack 3)
        (Utilities|Set|Add _hashsetepicattack_2 25)))))

(fn TakeDamage
  (params (Damage :type Float%20%28single-precision%29%20%28by%20ref%29))
  (Variables|Default|SetIsEggLife false)
  (bind _array_element (Utilities|Array|ForEachLoopwithBreak (Variables|Default|GetSuperEggs) :!label _label)
    (:LoopBody
      (if (Utilities|IsValid _array_element)
        (Variables|Default|SetIsEggLife true)
        (goto _label Break)))
    (:Completed
      (if (not (Variables|Default|GetIsEggLife))
        (CallFunction|CheckOpotinityEpicAttack)
        (|CallParentFunction Damage)
        (return)))))

(fn Killed
  (bind _returnvalue (Transformation|GetActorLocation))
  (bind _bp_gamemod (Variables|Default|GetBP_GameMod))
  (Effects|SpawnEmitteratLocation "/Game/Assets/Particles/P_Pixel_Explosion_Enemy.P_Pixel_Explosion_Enemy" (Transformation|GetActorLocation))
  (Default|EnemyKilled _bp_gamemod)
  (Default|SetScore _bp_gamemod (Variables|Default|GetEnemyScore))
  (Default|CameraShake _bp_gamemod "/Game/Blueprints/CamShake/BP_CamShake.BP_CamShake_C" _returnvalue)
  (Audio|PlaySoundatLocation 0 _returnvalue "0, 0, 0" 1.0 1.0 0.0 0 0 0)
  (Default|CallOnDied)
  (Actor|DestroyActor))

(fn ChangeWingsSkin
  (params (NewParam :type Linear%20Color%20Structure :default "(R=1.000000,G=1.000000,B=1.000000,A=1.000000)"))
  (for _array_element (Variables|Default|GetWingsMaterials)
    (Rendering|Material|SetVectorParameterValue _array_element "Color" NewParam :!class /Script/Engine.MaterialInstanceDynamic)))