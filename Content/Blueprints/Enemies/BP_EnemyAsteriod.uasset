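; Asteroid enemy actor that flies by projectile movement and awards score to the game mode when killed.
; On BeginPlay it calls ChangeSkin, then randomizes its speed and per-axis mesh scale within set ranges for variety.
; Killed adds score and camera shake through BP_GameMode, plays explosion effects and destroys the actor.
; Tick accumulates lifetime and silently destroys the asteroid once its TTL expires.
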(event EventBeginPlay
  (bind _projectilemovement (Variables|Default|GetProjectileMovement))
  (bind _minscale (Variables|Default|GetMinScale))
  (bind _maxscale (Variables|Default|GetMaxScale))
  (bind _returnvalue (Math|Random|RandomFloatinRange _minscale _maxscale))
  ;[1 1 1] Start
  (CallFunction|ChangeSkin)
  (bind _asbp_game_mode (Utilities|Casting|CastToBP_GameMode (Game|GetGameMode)))
  (Variables|Default|SetBP_GameMod _asbp_game_mode)
  (bind _output_get (Variables|Default|SetMoveSpeed (Math|Random|RandomFloatinRange (Variables|Default|GetMinSpeed) (Variables|Default|GetMaxSpeed))))
  (bind _output_get_2 (Variables|/Script/Engine.ProjectileMovementComponent|SetMaxSpeed _projectilemovement _output_get))
  (Variables|/Script/Engine.ProjectileMovementComponent|SetInitialSpeed _projectilemovement _output_get_2)
  (Transformation|SetWorldScale3D (Variables|Default|GetStaticMesh) (Math|Vector|MakeVector _returnvalue _returnvalue _returnvalue)))

(event EventKilled
  (bind _returnvalue (Transformation|GetActorLocation))
  (bind _bp_gamemod (Variables|Default|GetBP_GameMod))
  ;[1 1 1] Killed
  (Default|SetScore _bp_gamemod (Variables|Default|GetEnemyScore))
  (Default|CameraShake _bp_gamemod (Variables|Default|GetShake) _returnvalue)
  (Effects|SpawnEmitteratLocation "/Game/Assets/StarterContent/Particles/P_Explosion.P_Explosion" _returnvalue)
  (Audio|PlaySoundatLocation 0 _returnvalue "0, 0, 0" 1.0 1.0 0.0 0 0 0)
  (Actor|DestroyActor))

(event EventTick
  (params (DeltaSeconds :type Float%20%28single-precision%29))
  ;[1 1 1] Update
  (if (>= (Variables|Default|GetCurrentTime) (Variables|Default|GetTTL))
    (Actor|DestroyActor)
    (else
      (Variables|Default|SetCurrentTime (+ DeltaSeconds (Variables|Default|GetCurrentTime))))))

(fn ConstructionScript
  (|CallParentFunction))